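; BP_TargetBase is a shootable target that is either static or moving, with moving ones tinted orange.
; Moving targets oscillate around their spawn position along Direction on a sine wave, paced by the manager's speed multiplier.
; SizeMultiplier shrinks the target and raises its score, and movement adds a speed-based bonus.
; When shot, it reports points to the manager, requests a new target and destroys itself.
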(event Custom|OnShot
  (Variables|Default|SetMoveMultiplier (Math|Float|SelectFloat (+ (Variables|/Game/Assets/BP_ArenaManager.BP_ArenaManager_C|GetSpeedMultiplier (Variables|Default|GetManager)) 1.0) 1.0 (Variables|Default|GetbIsMoving)))
  (Default|AddScore (Variables|Default|GetManager) (* (* 1e+01 (Variables|Components|GetSizeMultiplier)) (Variables|Default|GetMoveMultiplier)))
  (Default|SpawnTarget (Variables|Default|GetManager))
  (Actor|DestroyActor))

(event EventTick
  (params (DeltaSeconds :type Float%20%28single-precision%29))
  (if (Variables|Default|GetbIsMoving)
    (bind _output_get (Variables|Default|SetPhase (+ (* (* DeltaSeconds 1.5) (Variables|/Game/Assets/BP_ArenaManager.BP_ArenaManager_C|GetSpeedMultiplier (Variables|Default|GetManager))) (Variables|Default|GetPhase))))
    (Transformation|SetActorLocation (+ (Variables|Default|GetOrigin) (* (Variables|Default|GetDirection) (* (Math|Trig|Sin(Radians) _output_get) (Variables|Default|GetAmplitude)))) false false)))

(event EventBeginPlay
  (bind _sizemultiplier (Variables|Components|GetSizeMultiplier))
  (bind _returnvalue (/ 1.5 _sizemultiplier))
  (Transformation|SetActorScale3D (Math|Vector|MakeVector _returnvalue _returnvalue _returnvalue))
  (Variables|Default|SetOrigin (Transformation|GetActorLocation))
  (if (Variables|Default|GetbIsMoving)
    (Rendering|Material|SetMaterial (Variables|Default|GetBody) 0 "/Game/Assets/M_TargetOrange.M_TargetOrange")))

(fn ConstructionScript)