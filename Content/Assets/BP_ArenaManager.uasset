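; BP_ArenaManager runs a target arena, creating the HUD, populating targets and tracking the score.
; On BeginPlay, StartRun adds WBP_HUD to the viewport and spawns a batch of BP_TargetBase actors at random points and sizes inside SpawnVolume.
; SpawnTarget recursively retries when collision blocks a spawn, then gives each target a reference back to the manager.
; AddScore adds rounded points to Score.
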(event EventBeginPlay
  (CallFunction|StartRun))

(event Collision|EventActorBeginOverlap
  (params (OtherActor :type Actor%20Object%20Reference)))

(event EventTick
  (params (DeltaSeconds :type Float%20%28single-precision%29)))

(fn ConstructionScript)

(fn SpawnTarget
  (bind _spawnvolume (Variables|Default|GetSpawnVolume))
  (bind _returnvalue (Game|SpawnActorfromClass "/Game/Assets/BP_TargetBase.BP_TargetBase_C" (Math|Transform|MakeTransform (Math|Random|RandomPointinBoundingBox (Transformation|GetWorldLocation _spawnvolume) (Components|Box|GetScaledBoxExtent _spawnvolume)) "0, 0, 0" "1.000000,1.000000,1.000000") "AdjustIfPossibleButDontSpawnIfColliding" "MultiplyWithRoot" 0 (Math|Random|RandomFloatinRange 1.0 2.5) 0))
  (Utilities|IsValid _returnvalue
    (:Is%20Valid
      (Variables|/Game/Assets/BP_TargetBase.BP_TargetBase_C|SetManager _returnvalue self))
    (:Is%20Not%20Valid
      (CallFunction|SpawnTarget))))

(fn StartRun
  (bind _returnvalue (UserInterface|CreateWidget "/Game/Assets/WBP_HUD.WBP_HUD_C" (Game|GetPlayerController 0)))
  (UserInterface|Viewport|AddtoViewport _returnvalue 0)
  (for _index (range 0 15)
    (CallFunction|SpawnTarget)))

(fn AddScore
  (params (Points :type Float%20%28double-precision%29))
  (Variables|Default|SetScore (+ (Math|Float|Round Points) (Variables|Default|GetScore))))